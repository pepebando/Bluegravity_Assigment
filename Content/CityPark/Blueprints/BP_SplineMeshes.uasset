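; BP_SplineMeshes lays a chosen mesh along a spline as deformed spline mesh segments, built in the construction script through the Wire graph.
; SplineMeshVar selects either one segment per pair of spline points or segments at a fixed Spacing along the spline's length.
; Each segment gets two materials, with tangents taken from the points or, in spacing mode, from spline direction scaled by Spacing plus TangentScaleAdd.
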(fn ConstructionScript
  (|Wire))